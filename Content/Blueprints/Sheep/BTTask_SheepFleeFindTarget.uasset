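; Behavior tree task that picks a flee destination for a sheep AI and writes it to the PatrolLocation blackboard key.
; FleeAlgorithm selects one of three methods, all scaled by a blackboard sphere radius: closest sphere point, forward projection onto the navmesh, or random reachable point around the sheep.
; The closest-point method returns the center-to-sheep direction times radius, without adding the center back.
; It fails for non-sheep pawns.
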(event `self.ReceiveExecuteAI`
  (params (OwnerController :type "AIController Object Reference") (ControlledPawn :type "Pawn Object Reference"))
  (bind _assheep_aicharacter_bp (cast `/Game/Blueprints/Sheep/SheepAICharacter_BP` ControlledPawn)
    (:`then`
      (switch `/Game/Blueprints/Sheep/FleeEnumeration` (`self.FleeAlgorithm`)
        (:`NewEnumerator0`
          (set `self.FleePosition` (`self.GetNewFleeLocationClosestSphere` _assheep_aicharacter_bp)))
        (:`NewEnumerator1`
          (set `self.FleePosition` (`self.GetNewFreeLocationForwardVector` _assheep_aicharacter_bp)))
        (:`NewEnumerator2`
          (set `self.FleePosition` (`self.GetNewFleeLocationRandomSphereFromPosition` _assheep_aicharacter_bp))))
      (`BTFunctionLibrary.SetBlackboardValueAsVector` (`self.PatrolLocation`) (`self.FleePosition`))
      (`self.FinishExecute` true))
    (:`CastFailed`
      (`self.FinishExecute` false))))

(fn `GetNewFleeLocationClosestSphere`
  (params (Pawn :type "Pawn Object Reference"))
  (returns (Location :type "Vector Structure"))
  (return (* (`KismetMathLibrary.Normal` (- (`Actor.K2_GetActorLocation` Pawn) (`NavigationSystemV1.K2_ProjectPointToNavigation` (`BTFunctionLibrary.GetBlackboardValueAsVector` (`self.SphereLocationKey`)) null "/Script/AIModule.NavFilter_AIControllerDefault"))) (`BTFunctionLibrary.GetBlackboardValueAsFloat` (`self.SphereRadiusKey`)))))

(fn `GetNewFleeLocationRandomSphereFromPosition`
  (params (Pawn :type "Pawn Object Reference"))
  (returns (Location :type "Vector Structure"))
  (return (`NavigationSystemV1.K2_GetRandomReachablePointInRadius` (`Actor.K2_GetActorLocation` Pawn) (`BTFunctionLibrary.GetBlackboardValueAsFloat` (`self.SphereRadiusKey`)) null null)))

(fn `GetNewFreeLocationForwardVector`
  (params (Pawn :type "Pawn Object Reference"))
  (returns (Location :type "Vector Structure"))
  (return (`NavigationSystemV1.K2_ProjectPointToNavigation` (+ (* (`Actor.GetActorForwardVector` Pawn) (`BTFunctionLibrary.GetBlackboardValueAsFloat` (`self.SphereRadiusKey`))) (`Actor.K2_GetActorLocation` Pawn)))))