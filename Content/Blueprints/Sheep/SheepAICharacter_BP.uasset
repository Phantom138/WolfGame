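; Sheep AI character that patrols within an assigned sphere and flees from wolves or dying sheep.
; On BeginPlay it reads the patrol radius and center from its assigned sphere, then has its SheepAI controller initialize the blackboard, printing a warning if no sphere is set.
; Flee events set blackboard bools for hearing a wolf or a sheep death.
; The death event destroys the actor after a short delay.
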(event `self.ReceiveBeginPlay`
  (bind _returnvalue (`self.GetComponentByClass` (`self.SphereComponent`) "/Script/Engine.SphereComponent"))
  ;[1 1 1] Get the radius and location from the Sphere Component that was attached
  (if (`KismetSystemLibrary.IsValid` (`self.SphereComponent`))
    (set `self.Patrol Radius` (`SphereComponent.GetScaledSphereRadius` _returnvalue))
    (set `self.PatrolSphereCenter` (`SceneComponent.K2_GetComponentLocation` _returnvalue))
    (bind _assheep_ai_controller_bp (cast `/Game/Blueprints/Sheep/SheepAI_Controller_BP` (`self.GetController`))
      (:`then`
        (`/Game/Blueprints/Sheep/SheepAI_Controller_BP.Initialize Blackboard` _assheep_ai_controller_bp))
      (:`CastFailed`
        (`KismetSystemLibrary.PrintString` "Cast failed !!" true true (struct :`R` 1.0 :`G` 0.013872 :`A` 1.0))))
    (else
      (`KismetSystemLibrary.PrintString` (`KismetStringLibrary.Concat_StrStr` "The sheep" (`KismetSystemLibrary.GetDisplayName` (`self.GetOwner`)) "is not in a sphere box component. It won't work!!!. \nMake sure the sheep is inside a ShapeBox_BP component!") true true (struct :`R` 1.0 :`B` 0.035222 :`A` 1.0) 1000.0))))

(event `DieEvent`
  ;[1 1 1] Sheep gets killed
  (`KismetSystemLibrary.Delay` 0.75)
  (`self.K2_DestroyActor`))

(event `Sheep Flee Hear Wolf`
  ;[1 0.08646 0.08646] Sheep Event to flee/run when wolf
  (bind _assheep_ai_controller_bp (cast `/Game/Blueprints/Sheep/SheepAI_Controller_BP` (`self.GetController`)))
  (`BlackboardComponent.SetValueAsBool` (`AIController.Blackboard` _assheep_ai_controller_bp) (`self.IsFleeingFromWolfKey`) true))

(event `Sheep Flee Sheep Dies`
  ;[0 0.9859 1] Shep Event to flee/run from other sheep dead
  (bind _assheep_ai_controller_bp (cast `/Game/Blueprints/Sheep/SheepAI_Controller_BP` (`self.GetController`)))
  (`BlackboardComponent.SetValueAsBool` (`AIController.Blackboard` _assheep_ai_controller_bp) (`self.isFleeingFromDeadSheepKey`) true))

(fn `UserConstructionScript`)