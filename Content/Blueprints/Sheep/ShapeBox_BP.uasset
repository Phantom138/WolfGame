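; ShapeBox_BP is an actor apparently meant to define a patrol area for sheep AI, but its logic is unwired and BeginPlay does nothing.
; The disconnected graph finds SheepAICharacter_BP actors overlapping CollisionComponent and prints their count.
; It would copy the sphere's scaled radius and the box actor's location into each sheep's patrol settings, printing an error if the component is not a sphere.
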(event `self.ReceiveBeginPlay`)

(fn `UserConstructionScript`)