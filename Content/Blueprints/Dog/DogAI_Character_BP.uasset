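; Dog AI character that catches the player and triggers game over.
; Capsule overlap with a third-person character that is not a sheep immediately fires GameOver, which disables input, calls GameLost on the player and restarts the game after a delay.
; End overlap clears the caught flag, while the timed-catch check in Tick leads to no action.
; A helper function sets the dog's walk speed.
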(event `self.ReceiveTick`
  (params (DeltaSeconds :type "Float (single-precision)"))
  (if (`self.isPlayerCaught?`)
    (if (> (- (`GameplayStatics.GetTimeSeconds`) (`self.caughtTime`)) (`self.timeToCatch`))
      _)))

(event `GameOver`
  ;[1 1 1] GameOver
  (`self.DisableInput` (`GameplayStatics.GetPlayerController` 0))
  (bind _asbp_third_person_character (cast `/Game/ThirdPerson/Blueprints/BP_ThirdPersonCharacter` (`GameplayStatics.GetPlayerPawn` 0)))
  (`/Game/ThirdPerson/Blueprints/BP_ThirdPersonCharacter.GameLost` _asbp_third_person_character)
  (`KismetSystemLibrary.Delay` 5.0)
  (bind _asgame_mode (cast `GameMode` (`GameplayStatics.GetGameMode`)))
  (`GameMode.RestartGame` _asgame_mode))

(event `self.Capsule.OnComponentBeginOverlap`
  (params (OverlappedComponent :type "PrimitiveComponent Object Reference") (OtherActor :type "Actor Object Reference") (OtherComp :type "PrimitiveComponent Object Reference") (OtherBodyIndex :type Integer) (bFromSweep :type Boolean) (SweepResult :type "HitResult Structure (by ref)"))
  (bind _asbp_third_person_character (cast `/Game/ThirdPerson/Blueprints/BP_ThirdPersonCharacter` OtherActor))
  (if (not (`/Game/ThirdPerson/Blueprints/BP_ThirdPersonCharacter.isSheep?` _asbp_third_person_character))
    (if (not (`self.isPlayerCaught?`))
      (set `self.caughtTime` (`GameplayStatics.GetTimeSeconds`))
      (set `self.isPlayerCaught?` true)
      (`self.GameOver`))))

(event `self.Capsule.OnComponentEndOverlap`
  (params (OverlappedComponent :type "PrimitiveComponent Object Reference") (OtherActor :type "Actor Object Reference") (OtherComp :type "PrimitiveComponent Object Reference") (OtherBodyIndex :type Integer))
  (cast `/Game/ThirdPerson/Blueprints/BP_ThirdPersonCharacter` OtherActor)
  (set `self.isPlayerCaught?` false)
  (`KismetSystemLibrary.PrintString` "Not caught"))

(fn `UpdateWalkSpeed`
  (params (NewWalkSpeed :type "Float (double-precision)"))
  (set `CharacterMovementComponent.MaxWalkSpeed` NewWalkSpeed (`self.CharacterMovement`)))

(fn `UserConstructionScript`)