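; AI controller for the dog that runs its behavior tree and reacts to seeing or hearing actors tagged Player.
; Successful perception updates feed separate hearing and sight handlers that write to the Blackboard.
; Hearing stores the sound location and sets an investigation flag, which a timer is set to clear.
; Sight stores the enemy and sets a line-of-sight flag that this controller never clears, with debug output throughout.
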(event `self.ReceivePossess`
  (params (PossessedPawn :type "Pawn Object Reference"))
  (`self.RunBehaviorTree` "/Game/Blueprints/Dog/DogAI_BehaviourTree.DogAI_BehaviourTree"))

(event `self.AIPerception.OnTargetPerceptionUpdated`
  (params (Actor :type "Actor Object Reference") (Stimulus :type "AIStimulus Structure"))
  (if (and (`self.ActorHasTag` Actor "Player") (`.bSuccessfullySensed` (break `AIStimulus` Stimulus)))
    (`self.HandleSoundSense` Stimulus)
    (`self.HandleVisionSense` Stimulus Actor)
    (`KismetSystemLibrary.PrintString` "Hello")))

(event `Stop Investigation`
  (`BlackboardComponent.SetValueAsBool` (`self.Blackboard`) (`self.IsInvestigation`) false)
  (`KismetSystemLibrary.PrintString` "Done Investigation" true true (struct :`R` 1.0 :`G` 0.570049 :`B` 0.206088 :`A` 1.0) 2.0 "Investigation"))

(fn `HandleSoundSense`
  (params (Stimulus :type "AIStimulus Structure (by ref)"))
  (bind (_age _expirationage _strength _stimuluslocation) (break `AIStimulus` (`local.Stimulus`)))
  (bind _returnvalue (`AIPerceptionSystem.GetSenseClassForStimulus` Stimulus))
  (if (== _returnvalue "/Script/AIModule.AISense_Hearing")
    (`BlackboardComponent.SetValueAsVector` (`self.Blackboard`) (`self.WolfSoundLocationKey`) _stimuluslocation)
    (`KismetSystemLibrary.PrintString` "Sound was sensed" true true (struct :`R` 1.0 :`G` 0.00786 :`A` 1.0) 3.0 "Sound Sensed")
    (`KismetSystemLibrary.DrawDebugCircle` _stimuluslocation 20.0 12 (struct :`R` 1.0 :`G` 0.008675 :`B` 0.445805 :`A` 1.0) 20.0 5.0)
    (`BlackboardComponent.SetValueAsBool` (`self.Blackboard`) (`self.IsInvestigation`) true)
    (`KismetSystemLibrary.K2_SetTimer` null "Stop Investigation" (`self.TimeToInvestigate`))))

(fn `HandleVisionSense`
  (params (Stimulus :type "AIStimulus Structure (by ref)") (Actor :type "Actor Object Reference"))
  (bind _blackboard (`self.Blackboard`))
  (bind _returnvalue (`AIPerceptionSystem.GetSenseClassForStimulus` Stimulus))
  (if (== _returnvalue "/Script/AIModule.AISense_Sight")
    (`BlackboardComponent.SetValueAsBool` _blackboard (`self.HasLineOfSightKey?`) true)
    (`BlackboardComponent.SetValueAsObject` _blackboard (`self.EnemyActorKey`) Actor)
    (`KismetSystemLibrary.PrintString` "Vision detcted!")))

(fn `UserConstructionScript`)